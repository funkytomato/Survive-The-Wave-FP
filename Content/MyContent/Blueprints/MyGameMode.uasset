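; Game mode Blueprint that defines a level timer, a Kudos score and an exit gate that opens at the Kudos cap.
; LevelTimer counts seconds and minutes, while CalculateKudos adds Kudos per captured power point, clamps the total and calls EnableLevelGate to open or close the gate.
; The setup for one-second looping timers and the gate reference is disconnected from BeginPlay, so it never runs.
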(event EventBeginPlay
  ;[1 1 1] Start Level Timer and Kudos Counter
)

(fn ConstructionScript)

(fn LevelTimer
  (Variables|Time|SetSeconds (+ (Variables|Time|GetSeconds) 1))
  (if (> (Variables|Time|GetSeconds) 59)
    (Variables|Time|SetMinutes (+ (Variables|Time|GetMinutes) 1))
    (Variables|Time|SetSeconds 0)))

(fn CalculateKudos
  (Variables|PowerPoint|SetKudos (Math|Integer|Clamp(Integer) (+ (Variables|PowerPoint|GetKudos) (* (Variables|PowerPoint|GetPowerPointsCaptured) (Variables|PowerPoint|GetPowerPointKudos))) 0 (Variables|PowerPoint|GetMaxKudos)))
  (CallFunction|EnableLevelGate)
  (return))

(fn EnableLevelGate
  (bind _exitgateref (Variables|Default|GetExitGateRef))
  ;[1 1 1] Enable End of Level Gate when Kudos reaches 1000
  (if (>= (Variables|PowerPoint|GetKudos) (Variables|PowerPoint|GetMaxKudos))
    (Default|CallLevelGateOpen _exitgateref)
    (else
      (Default|CallLevelGateClose _exitgateref)))
  (return))