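; Game mode that runs wave-based enemy levels, tracking score, experience, kills and level time, and creating the HUD.
; Level and wave data tables set the wave count and enemy pool, with randomized counts as fallback for missing wave rows.
; Random active spawners queue pooled enemies up to a cap, refilling on kills while enough remain.
; A cleared wave ends and starts a timed transition to the next, until the level's wave limit.
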(event Custom|Timer
  (CallFunction|LevelTimer)
  (Default|UpdateTme (Variables|/Game/MyContent/UI/HUD/STW_HUD.STW_HUD_C|GetW_Time (Variables|Default|GetHUD))))

(event Custom|ResetGameStats
  (params (ExperiencePoints :type Integer) (Rank :type Integer) (Lives :type Integer))
  (Variables|GamesStats|SetExperience%20Points ExperiencePoints)
  (Variables|GamesStats|SetRank Rank)
  (Variables|GamesStats|SetLives Lives))

(event Custom|InitialiseGameStart
  (bind _asgame_info_instance (Utilities|Casting|CastToGameInfoInstance (Game|GetGameInstance)))
  (Default|ResetPlayerInfo _asgame_info_instance))

(event EventBeginPlay
  (CallFunction|LoadLevelData)
  (Utilities|Time|SetTimerbyEvent (delegate Custom|Timer) 1.0 true)
  (bind _returnvalue (UserInterface|CreateWidget "/Game/MyContent/UI/HUD/STW_HUD.STW_HUD_C"))
  (bind _output_get (Variables|Default|SetHUD _returnvalue))
  (UserInterface|Viewport|AddtoViewport _output_get 0)
  (Input|SetInputModeGameOnly (Game|GetPlayerController 0) false)
  (CallFunction|NewWave))

(fn ConstructionScript)

(fn GetSpawners
  (bind _outactors (Actor|GetAllActorsOfClass "/Game/MyContent/WaveSpawner/EnemySpawner.EnemySpawner_C"))
  (bind _output_get (Variables|WaveSpawner|SetSpawners _outactors))
  (bind _output_get_2 (LocalVariables|SetLocal_Spawners _output_get))
  (for _array_element _output_get_2
    (if (not (Variables|/Game/MyContent/WaveSpawner/EnemySpawner.EnemySpawner_C|GetIsOn _array_element))
      (Utilities|Array|RemoveItem (Variables|WaveSpawner|GetSpawners) _array_element))))

(fn StartWave
  (bind _sum (CallFunction|GetPoolSize))
  (bind _enemymaxcount (Variables|WaveSpawner|GetEnemyMaxCount))
  (bind _returnvalue (Math|Integer|Min(Integer) _sum _enemymaxcount))
  (bind _returnvalue_2 (- _returnvalue 1))
  (CallFunction|LoadLevelData)
  (CallFunction|BuildEnemyPool)
  (for _index (range 0 _returnvalue_2)
    (Development|PrintString (Utilities|String|ToString(Integer) _index))
    (Default|AddEnemytoQueue (.OutItem (Utilities|Array|Random (Variables|WaveSpawner|GetSpawners))) (CallFunction|GetEnemyfromPool)))
  (Development|PrintString (Utilities|String|ToString(Text) (Utilities|Text|FormatText "{Enemy Count}" _returnvalue_2))))

(fn EndWave
  (Math|Integer|IncrementInt (Variables|GamesStats|GetWaves%20Passed)
    (:%20%20
      (Default|CallOnEndWave))))

(fn BuildEnemyPool
  (bind _returnvalue (Utilities|GetDataTableRow "/Game/MyContent/WaveSpawner/WavePoolData.WavePoolData" (Utilities|String|StringToName (Utilities|String|ToString(Integer) (Variables|WaveSpawner|GetWave%20ID))))
    (:then
      (Variables|WaveSpawner|SetEnemyPool (Utilities|Struct|BreakF_WaveStruct _returnvalue))
      (Variables|WaveSpawner|SetEnemyRemaining (CallFunction|GetPoolSize)))
    (:RowNotFound
      (Utilities|Map|Add (Variables|WaveSpawner|GetEnemyPool) (Variables|Default|GetEnemyClassA) (Math|Random|RandomIntegerinRange 10 (* (Variables|WaveSpawner|GetWaveNumber) 5)))
      (Utilities|Map|Add (Variables|WaveSpawner|GetEnemyPool) (Variables|Default|GetEnemyClassB) (Math|Random|RandomIntegerinRange 5 (* (Variables|WaveSpawner|GetWaveNumber) 3)))
      (Variables|WaveSpawner|SetEnemyRemaining (CallFunction|GetPoolSize)))))

(fn GetPoolSize
  (bind _values (Utilities|Map|Values (Variables|WaveSpawner|GetEnemyPool)))
  (for _array_element _values
    (LocalVariables|SetLocal_Sum (+ (LocalVariables|GetLocal_Sum) _array_element)))
  (return (LocalVariables|GetLocal_Sum)))

(fn GetEnemyfromPool
  (bind _keys (Utilities|Map|Keys (Variables|WaveSpawner|GetEnemyPool)))
  (bind _output_get (LocalVariables|SetLocalClassChoice (.OutItem (Utilities|Array|Random _keys))))
  (if (> (- (.Value (Utilities|Map|Find (Variables|WaveSpawner|GetEnemyPool) _output_get)) 1) 0)
    (Utilities|Map|Add (Variables|WaveSpawner|GetEnemyPool) (LocalVariables|GetLocalClassChoice) (- (.Value (Utilities|Map|Find (Variables|WaveSpawner|GetEnemyPool) _output_get)) 1))
    (return (LocalVariables|GetLocalClassChoice))
    (else
      (Utilities|Map|Remove (Variables|WaveSpawner|GetEnemyPool) (LocalVariables|GetLocalClassChoice))
      (return (LocalVariables|GetLocalClassChoice)))))

(fn NewWave
  (Variables|GamesStats|SetEnemyKills 0)
  (if (< (Variables|WaveSpawner|GetWaveNumber) (Variables|GamesStats|GetWaves%20This%20Level))
    (Math|Integer|IncrementInt (Variables|WaveSpawner|GetWaveNumber)
      (:%20%20
        (CallFunction|GetSpawners)
        (CallFunction|StartWave)
        (Default|CallOnNewWave (Variables|WaveSpawner|GetWaveNumber) (Variables|WaveSpawner|GetEnemyRemaining))))))

(fn OnEnemyDefeated
  (params (Points :type Integer) (Experience :type Integer))
  (Math|Integer|IncrementInt (Variables|GamesStats|GetEnemyKills)
    (:%20%20
      (Variables|GamesStats|SetScore (+ (Variables|GamesStats|GetScore) Points))
      (Variables|GamesStats|SetExperience%20Points (+ (Variables|GamesStats|GetExperience%20Points) Experience))
      (bind _result (Math|Integer|DecrementInt (Variables|WaveSpawner|GetEnemyRemaining))
        (:%20%20
          (Default|CallOnEnemyKilled (Variables|WaveSpawner|GetEnemyRemaining))
          (if (< _result (Variables|WaveSpawner|GetEnemyMaxCount))
            (if (<= (Variables|WaveSpawner|GetEnemyRemaining) 0)
              (CallFunction|EnterTransition 5.0))
            (else
              (Default|AddEnemytoQueue (.OutItem (Utilities|Array|Random (Variables|WaveSpawner|GetSpawners))) (CallFunction|GetEnemyfromPool)))))))))

(fn EnterTransition
  (params (TransitionPeriod :type Float%20%28single-precision%29))
  (bind _returnvalue (Utilities|Time|SetTimerbyFunctionName 0 "NewWave" TransitionPeriod))
  (Variables|WaveSpawner|SetTransitionTimer _returnvalue)
  (Utilities|Casting|CastToSTW_PlayerCharacter (Game|GetPlayerCharacter 0))
  (CallFunction|EndWave))

(fn LevelTimer
  (Variables|GamesStats|SetSeconds (+ (Variables|GamesStats|GetSeconds) 1))
  (if (> (Variables|GamesStats|GetSeconds) 59)
    (Variables|GamesStats|SetMinutes (+ (Variables|GamesStats|GetMinutes) 1))
    (Variables|GamesStats|SetSeconds 0)))

(fn LoadLevelData
  (bind _asgame_info_instance (Utilities|Casting|CastToGameInfoInstance (Game|GetGameInstance)))
  (bind _levelname (Default|GetCurrentLevel _asgame_info_instance))
  (bind _returnvalue (Utilities|GetDataTableRow "/Game/MyContent/WaveSpawner/LevelPoolData.LevelPoolData" _levelname)
    (:then
      (Variables|GamesStats|SetCurrentLevelNo (.LevelNo (Utilities|Struct|BreakF_LevelStruct _returnvalue)))
      (Variables|GamesStats|SetWaves%20This%20Level (.WavesThisLevel (Utilities|Struct|BreakF_LevelStruct _returnvalue)))
      (Variables|WaveSpawner|SetWave%20ID (.WaveID (Utilities|Struct|BreakF_LevelStruct _returnvalue)))
      (Variables|WaveSpawner|SetEnemyRemaining (CallFunction|GetPoolSize))
      (return))))