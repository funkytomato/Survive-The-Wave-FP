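; Health and armour component that processes damage and health boosts for its owner, broadcasting health changes and death through dispatchers.
; Damage type casts route hits: scaled headshots bypass armour, scaled limb hits only hurt at zero armour without draining it, and other hits drain armour first.
; Non-player owners get a screen-projected popup, which shows remaining health rather than damage on default hits.
; The armour boost handler is empty.
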(event Custom|RecieveDamage_Event
  (params (Damage :type Float%20%28double-precision%29) (DamageType :type Damage%20Type%20Object%20Reference) (InstigatedBy :type Controller%20Object%20Reference) (DamageCauser :type Actor%20Object%20Reference))
  (bind _asdamage_type_headshot (Utilities|Casting|CastToDamageTypeHeadshot DamageType)
    (:then
      ;[1 1 1] Apply Headshot increased Damage.  Show bloodscreen!!!!
      (bind _currenthealth (CallFunction|DecreaseHealth (* (Variables|/Game/MyContent/Blueprints/Health/DamageTypeHeadshot.DamageTypeHeadshot_C|Getmultiplier _asdamage_type_headshot) Damage)))
      (Default|CallUpdateHealth _currenthealth (* (Variables|/Game/MyContent/Blueprints/Health/DamageTypeHeadshot.DamageTypeHeadshot_C|Getmultiplier _asdamage_type_headshot) Damage))
      ;[1 1 1] Display Damage Popup Widget
      (CallFunction|DisplayDamagePopup (* (Variables|/Game/MyContent/Blueprints/Health/DamageTypeHeadshot.DamageTypeHeadshot_C|Getmultiplier _asdamage_type_headshot) Damage)))
    (:CastFailed
      (bind _asdamage_type_limbs (Utilities|Casting|CastToDamageTypeLimbs DamageType)
        (:then
          ;[1 1 1] Apply Limbs decreased Damage.  Show bloodscreen!!!!
          (CallFunction|DecreaseArmour 0.0)
          (if (Variables|Default|GetnoArmour?)
            (bind _currenthealth_2 (CallFunction|DecreaseHealth (* (Variables|/Game/MyContent/Blueprints/Health/DamageTypeLimbs.DamageTypeLimbs_C|Getmultiplier _asdamage_type_limbs) Damage)))
            (Default|CallUpdateHealth _currenthealth_2 (* (Variables|/Game/MyContent/Blueprints/Health/DamageTypeLimbs.DamageTypeLimbs_C|Getmultiplier _asdamage_type_limbs) Damage))
            (CallFunction|DisplayDamagePopup (* (Variables|/Game/MyContent/Blueprints/Health/DamageTypeLimbs.DamageTypeLimbs_C|Getmultiplier _asdamage_type_limbs) Damage))))
        (:CastFailed
          ;[1 1 1] Apply default damage and reduce armour before health.  Show bloodscreen!!!!
          (CallFunction|DecreaseArmour Damage)
          (if (Variables|Default|GetnoArmour?)
            (bind _currenthealth_3 (CallFunction|DecreaseHealth Damage))
            (Default|CallUpdateHealth _currenthealth_3 Damage)
            (CallFunction|DisplayDamagePopup _currenthealth_3)))))))

(event Custom|HealthBoost_Event
  (params (healthBoost :type Float%20%28double-precision%29))
  ;[1 1 1] Increase Boost Event Dispatcher
  ;;[1 1 1] Increase Health
  (bind _currenthealth (CallFunction|IncreaseHealth healthBoost))
  ;;[1 1 1] Update Blood Screen
  (Default|CallUpdateHealth _currenthealth 0.0))

(event Custom|ArmorBoost_Event
  (params (boostAmount :type Float%20%28double-precision%29)))

(event EventBeginPlay
  ;[1 1 1] Recieved Damage Event Dispatcher
  (EventDispatchers|BindEventtoRecieveDamage (delegate Custom|RecieveDamage_Event))
  ;[1 1 1] Increase Boost Event Dispatcher
  (EventDispatchers|BindEventtoHealthBoost (delegate Custom|HealthBoost_Event))
  (EventDispatchers|BindEventtoArmorBoost (delegate Custom|ArmorBoost_Event)))

(fn IncreaseHealth
  (params (value :type Float%20%28double-precision%29))
  (bind _output_get (Variables|Default|SetHealth (Math|Float|Clamp(Float) (+ (Variables|Default|GetHealth) value) 0.0 (Variables|Default|GetMaxHealth))))
  (Variables|Default|SetIsDead? (not (> _output_get 0.0)))
  (return _output_get))

(fn DecreaseHealth
  (params (value :type Float%20%28double-precision%29))
  (bind _output_get (Variables|Default|SetHealth (Math|Float|Clamp(Float) (- (Variables|Default|GetHealth) value) 0.0 (Variables|Default|GetMaxHealth))))
  (bind _output_get_2 (Variables|Default|SetIsDead? (not (> _output_get 0.0))))
  (if _output_get_2
    (Default|CallIsDead))
  (return _output_get))

(fn DecreaseArmour
  (params (amount :type Float%20%28double-precision%29))
  (bind _output_get (Variables|Default|SetArmour (Math|Float|Clamp(Float) (- (Variables|Default|GetArmour) amount) 0.0 (Variables|Default|GetMaxArmour))))
  (Variables|Default|SetnoArmour? (== _output_get 0.0)))

(fn IncreaseArmour
  (params (amount :type Float%20%28double-precision%29))
  (bind _output_get (Variables|Default|SetArmour (Math|Float|Clamp(Float) (+ (Variables|Default|GetArmour) amount) 0.0 (Variables|Default|GetMaxArmour))))
  (Variables|Default|SetnoArmour? (not (> _output_get 0.0))))

(fn DisplayDamagePopup
  (params (DPS :type Float%20%28double-precision%29))
  (if (not (Variables|Default|GetIsPlayer?))
    (bind _returnvalue (UserInterface|CreateWidget "/Game/MyContent/UI/Damage/DamageRecieved_WBP.DamageRecieved_WBP_C" 0 false DPS))
    (UserInterface|Viewport|AddtoViewport _returnvalue 0)
    (bind _myowner (Variables|Default|GetMyOwner)
      (:then
        (Class|UserWidget|SetPositioninViewport _returnvalue (.ScreenPosition (Class|GameplayStatics|ProjectWorldtoScreen (Game|GetPlayerController 0) (Transformation|GetActorLocation _myowner) false)) true))
      (:else))))