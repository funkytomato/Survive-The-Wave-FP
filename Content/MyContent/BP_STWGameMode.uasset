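; Game mode for an enemy wave mode that creates the wave HUD and starts the first wave on BeginPlay.
; Each wave builds a class-to-count pool from a data table row keyed by wave number, with randomized scaling counts as fallback.
; Random active spawners receive enemies up to a cap, then refills as enemies die.
; Dispatchers report wave starts, kills and ends, and a timer launches the next wave after a clear.
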(event EventBeginPlay
  (bind _returnvalue (UserInterface|CreateWidget "/Game/MyContent/UI/W_WaveModeHUD.W_WaveModeHUD_C"))
  (bind _output_get (Variables|Default|SetHUD _returnvalue))
  (UserInterface|Viewport|AddtoViewport _output_get 0)
  (CallFunction|NewWave))

(fn ConstructionScript)

(fn GetSpawners
  (bind _outactors (Actor|GetAllActorsOfClass "/Game/MyContent/WaveSpawner/EnemySpawner.EnemySpawner_C"))
  (bind _output_get (Variables|Default|SetSpawners _outactors))
  (bind _output_get_2 (LocalVariables|SetLocal_Spawners _output_get))
  (for _array_element _output_get_2
    (if (not (Variables|/Game/MyContent/WaveSpawner/EnemySpawner.EnemySpawner_C|GetIsOn _array_element))
      (Utilities|Array|RemoveItem (Variables|Default|GetSpawners) _array_element))))

(fn StartWave
  (CallFunction|BuildEnemyPool)
  (for _index (range 0 (- (Math|Integer|Min(Integer) (CallFunction|GetPoolSize) (Variables|Default|GetEnemyMaxCount)) 1))
    (Default|AddEnemytoQueue (.OutItem (Utilities|Array|Random (Variables|Default|GetSpawners))) (CallFunction|GetEnemyfromPool))))

(fn EndWave
  (Default|CallOnEndWave))

(fn BuildEnemyPool
  (bind _returnvalue (Utilities|GetDataTableRow "/Game/MyContent/WaveSpawner/WavePoolData.WavePoolData" (Utilities|String|StringToName (Utilities|String|ToString(Integer) (Variables|Default|GetWaveNumber))))
    (:then
      (Variables|Default|SetEnemyPool (Utilities|Struct|BreakF_WaveStruct _returnvalue))
      (Variables|Default|SetEnemyRemaining (CallFunction|GetPoolSize)))
    (:RowNotFound
      (Utilities|Map|Add (Variables|Default|GetEnemyPool) "/Game/MyContent/Enemy/Enemy_BP.Enemy_BP_C" (Math|Random|RandomIntegerinRange 10 (* (Variables|Default|GetWaveNumber) 5)))
      (Utilities|Map|Add (Variables|Default|GetEnemyPool) "/Game/MyContent/Enemy/Enemy_Child.Enemy_Child_C" (Math|Random|RandomIntegerinRange 5 (* (Variables|Default|GetWaveNumber) 3)))
      (Variables|Default|SetEnemyRemaining (CallFunction|GetPoolSize)))))

(fn GetPoolSize
  (bind _values (Utilities|Map|Values (Variables|Default|GetEnemyPool)))
  (for _array_element _values
    (LocalVariables|SetLocal_Sum (+ (LocalVariables|GetLocal_Sum) _array_element)))
  (return (LocalVariables|GetLocal_Sum)))

(fn GetEnemyfromPool
  (bind _keys (Utilities|Map|Keys (Variables|Default|GetEnemyPool)))
  (bind _output_get (LocalVariables|SetLocalClassChoice (.OutItem (Utilities|Array|Random _keys))))
  (if (> (- (.Value (Utilities|Map|Find (Variables|Default|GetEnemyPool) _output_get)) 1) 0)
    (Utilities|Map|Add (Variables|Default|GetEnemyPool) (LocalVariables|GetLocalClassChoice) (- (.Value (Utilities|Map|Find (Variables|Default|GetEnemyPool) _output_get)) 1))
    (return (LocalVariables|GetLocalClassChoice))
    (else
      (Utilities|Map|Remove (Variables|Default|GetEnemyPool) (LocalVariables|GetLocalClassChoice))
      (return (LocalVariables|GetLocalClassChoice)))))

(fn NewWave
  (Math|Integer|IncrementInt (Variables|Default|GetWaveNumber)
    (:%20%20
      (CallFunction|GetSpawners)
      (CallFunction|StartWave)
      (Default|CallOnNewWave (Variables|Default|GetWaveNumber) (Variables|Default|GetEnemyRemaining)))))

(fn OnEnemyDefeated
  (bind _result (Math|Integer|DecrementInt (Variables|Default|GetEnemyRemaining))
    (:%20%20
      (Default|CallOnEnemyKilled (Variables|Default|GetEnemyRemaining))
      (if (< _result (Variables|Default|GetEnemyMaxCount))
        (if (<= (Variables|Default|GetEnemyRemaining) 0)
          (CallFunction|EnterTransition 5.0))
        (else
          (Default|AddEnemytoQueue (.OutItem (Utilities|Array|Random (Variables|Default|GetSpawners))) (CallFunction|GetEnemyfromPool)))))))

(fn EnterTransition
  (params (TransitionPeriod :type Float%20%28single-precision%29))
  (bind _returnvalue (Utilities|Time|SetTimerbyFunctionName 0 "NewWave" TransitionPeriod))
  (Variables|Default|SetTransitionTimer _returnvalue)
  (CallFunction|EndWave))