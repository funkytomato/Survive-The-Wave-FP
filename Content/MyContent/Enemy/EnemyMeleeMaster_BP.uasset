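; Master Blueprint for melee enemies that toggles chase behaviour when attacks start and stop.
; It overrides the parent's Attack and AttackStop events to set a chasing flag and switch movement speed between chase and walk values.
; Both events mirror the state into the AI controller's blackboard IsChasing key.
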(event EventBeginPlay
  (|CallParentFunction) ; This node is disabled and will not be called.\nDrag off pins to build functionality.
)

(event EventTick
  (params (DeltaSeconds :type Float%20%28single-precision%29))
  (|CallParentFunction DeltaSeconds) ; This node is disabled and will not be called.\nDrag off pins to build functionality.
)

(event EventAttack
  ;[1 1 1] Start Chase
  (|CallParentFunction)
  (Variables|Default|SetIsChasing true)
  (Variables|/Script/Engine.CharacterMovementComponent|SetMaxWalkSpeed (Variables|Character|GetCharacterMovement) (Variables|Default|GetChaseSpeed))
  (AI|Components|Blackboard|SetValueasBool (AI|GetBlackboard (AI|GetAIController self)) (Utilities|Name|MakeLiteralName "IsChasing") true))

(event EventAttackStop
  ;[1 1 1] Stop Chase
  (|CallParentFunction)
  (Variables|Default|SetIsChasing false)
  (Variables|/Script/Engine.CharacterMovementComponent|SetMaxWalkSpeed (Variables|Character|GetCharacterMovement) (Variables|Default|GetWalkSpeed))
  (AI|Components|Blackboard|SetValueasBool (AI|GetBlackboard (AI|GetAIController self)) (Utilities|Name|MakeLiteralName "IsChasing") false))

(fn ConstructionScript
  (|CallParentFunction))