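; Master enemy character Blueprint that chases or attacks the player through an AI Blackboard TargetActor key, set and cleared by a proximity overlap that also swaps its material.
; Hitting the player deals fixed damage.
; Damage taken awards player XP on every hit, feeds the health component and briefly flashes an armoured or unarmoured material.
; The component's death event broadcasts point and experience values, then destroys the enemy.
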(event OnComponentBeginOverlap(AttackProximity)
  (params (OverlappedComponent :type Primitive%20Component%20Object%20Reference) (OtherActor :type Actor%20Object%20Reference) (OtherComp :type Primitive%20Component%20Object%20Reference) (OtherBodyIndex :type Integer) (bFromSweep :type Boolean) (SweepResult :type Hit%20Result%20Structure%20%28by%20ref%29))
  ;[1 1 1] Attack Player when within proximity
  (if (== OtherActor (Game|GetPlayerCharacter 0))
    (CallFunction|ChangeMaterial "/Game/MyContent/Materials/AttackMaterial.AttackMaterial")
    (AI|Components|Blackboard|SetValueasObject (AI|GetBlackboard (AI|GetAIController self)) (Utilities|Name|MakeLiteralName "TargetActor") OtherActor)))

(event OnComponentEndOverlap(AttackProximity)
  (params (OverlappedComponent :type Primitive%20Component%20Object%20Reference) (OtherActor :type Actor%20Object%20Reference) (OtherComp :type Primitive%20Component%20Object%20Reference) (OtherBodyIndex :type Integer))
  (bind _self self)
  (bind _returnvalue (AI|GetAIController _self))
  ;[1 1 1] Forget Player when left proximity
  (if (== OtherActor (Game|GetPlayerCharacter 0))
    (CallFunction|ChangeMaterial (Variables|Character|GetDefaultMaterialInstance))
    (Utilities|IsValid _returnvalue
      (:Is%20Valid
        (AI|Components|Blackboard|SetValueasObject (AI|GetBlackboard _returnvalue) (Utilities|Name|MakeLiteralName "TargetActor") 0)))))

(event Custom|Died
  ;[1 1 1] BeginPlay - Initialise Health Component, Bind Messages, Reference Default Material and Start Movement
  (Default|CallOnDestroyed (Variables|Character|GetPointValue) (Variables|Character|GetExperienceValue))
  (Actor|DestroyActor))

(event EventBeginPlay
  ;[1 1 1] BeginPlay - Initialise Health Component, Bind Messages, Reference Default Material and Start Movement
  (Variables|/Script/Engine.CharacterMovementComponent|SetMaxWalkSpeed (Variables|Character|GetCharacterMovement) (Variables|Chase|GetWalkSpeed))
  (Variables|/Game/MyContent/Blueprints/Health/Health_CBP.Health_CBP_C|SetMyOwner (Variables|Default|GetHealth_CBP) self)
  (Variables|Character|SetDefaultMaterialInstance (Rendering|Material|GetMaterial (Variables|Default|GetCone) 0))
  (AI|Components|Blackboard|SetValueasObject (AI|GetBlackboard (AI|GetAIController self)) (Utilities|Name|MakeLiteralName "TargetActor") 0)
  (EventDispatchers|BindEventtoIsDead (Variables|Default|GetHealth_CBP) (delegate Custom|Died)))

(event Collision|EventHit
  (params (MyComp :type Primitive%20Component%20Object%20Reference) (Other :type Actor%20Object%20Reference) (OtherComp :type Primitive%20Component%20Object%20Reference) (bSelfMoved :type Boolean) (HitLocation :type Vector :default "0, 0, 0") (HitNormal :type Vector :default "0, 0, 0") (NormalImpulse :type Vector :default "0, 0, 0") (Hit :type Hit%20Result%20Structure%20%28by%20ref%29))
  ;[1 1 1] On Hit Player
  (bind _asstw_player_character (Utilities|Casting|CastToSTW_PlayerCharacter Other))
  (Game|Damage|ApplyDamage _asstw_player_character 1e+01 0 self "/Game/MyContent/Blueprints/Health/DamageTypeLimbs.DamageTypeLimbs_C"))

(event Game|Damage|EventAnyDamage
  (params (Damage :type Float%20%28single-precision%29) (DamageType :type Damage%20Type%20Object%20Reference) (InstigatedBy :type Controller%20Object%20Reference) (DamageCauser :type Actor%20Object%20Reference))
  (bind _health_cbp (Variables|Default|GetHealth_CBP))
  ;[1 1 1] Recieve Damage
  (bind _asstw_player_character (Utilities|Casting|CastToSTW_PlayerCharacter (Game|GetPlayerCharacter 0)))
  (Default|AddXP (Variables|/Game/MyContent/Character/STW_PlayerCharacter.STW_PlayerCharacter_C|GetLevellingSystem _asstw_player_character) (Variables|Character|GetExperienceValue))
  (Default|RecieveDamageEvent _health_cbp Damage DamageType InstigatedBy DamageCauser)
  (bind _cone (Variables|Default|GetCone)
    (:then
      (if (Variables|/Game/MyContent/Blueprints/Health/Health_CBP.Health_CBP_C|GetnoArmour? _health_cbp)
        ;;[1 1 1] Show NoArmour Hits (Blood or Shrapnel)
        (Rendering|Material|SetMaterial _cone 0 "/Game/BallisticsVFX/DemoMap/Materials/MetalDull.MetalDull")
        (Utilities|FlowControl|Delay 0.8)
        (Rendering|Material|SetMaterial (Variables|Default|GetCone) 0 (Variables|Character|GetDefaultMaterialInstance))
        (else
          ;;[1 1 1] Show Armoured Hits (Shield)
          (Rendering|Material|SetMaterial _cone 0 "/Game/BallisticsVFX/DemoMap/Materials/ShieldEnergy2.ShieldEnergy2")
          (Utilities|FlowControl|Delay 0.5)
          (Rendering|Material|SetMaterial (Variables|Default|GetCone) 0 (Variables|Character|GetDefaultMaterialInstance)))))
    (:else)))

(fn ConstructionScript)

(fn ChangeMaterial
  (params (Material :type Material%20Interface%20Object%20Reference))
  (Rendering|Material|SetMaterial (Variables|Default|GetCone) 0 Material)
  (return))