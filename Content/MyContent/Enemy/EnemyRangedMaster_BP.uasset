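; Base ranged enemy Blueprint that fires CubitUniProjectile from its muzzle while attacking.
; Attack extends the parent event, switches movement to attack speed and starts a looping timer at FireRate that spawns projectiles with the enemy as instigator.
; AttackStop restores walk speed and clears the timer.
; A FireProjectile function duplicates the spawn logic but is not called in this file.
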(event Custom|FireTimer
  ;[1 1 1] Trigger Fire Projectile Timer
  (Game|SpawnActorfromClass "/Game/BallisticsVFX/FXSpawnerBlueprints/Projectiles/CubitUniProjectile.CubitUniProjectile_C" (Transformation|GetWorldTransform (Variables|Default|GetMuzzleScene)) "Undefined" "MultiplyWithRoot" 0 3e+04 true true false "NewEnumerator1" 0 "NewEnumerator0" true self))

(event EventBeginPlay
  (|CallParentFunction) ; This node is disabled and will not be called.\nDrag off pins to build functionality.
)

(event EventAttack
  ;[1 1 1] Ranged Attack - Run Enemy Ranged Behaviour Tree
  (|CallParentFunction)
  (Variables|Default|SetIsAttacking true)
  (Variables|/Script/Engine.CharacterMovementComponent|SetMaxWalkSpeed (Variables|Character|GetCharacterMovement) (Variables|Default|GetAttackSpeed))
  (bind _returnvalue (Utilities|Time|SetTimerbyEvent (delegate Custom|FireTimer) (Variables|Default|GetFireRate) true))
  (Variables|Default|SetFireProjectileTimerRef _returnvalue))

(event EventAttackStop
  ;[1 1 1] Stop Ranged Attack
  (|CallParentFunction)
  (Variables|Default|SetIsAttacking false)
  (Variables|/Script/Engine.CharacterMovementComponent|SetMaxWalkSpeed (Variables|Character|GetCharacterMovement) (Variables|Default|GetWalkSpeed))
  (Utilities|Time|ClearandInvalidateTimerbyHandle (Variables|Default|GetFireProjectileTimerRef)))

(fn ConstructionScript
  (|CallParentFunction))

(fn FireProjectile
  (Game|SpawnActorfromClass "/Game/BallisticsVFX/FXSpawnerBlueprints/Projectiles/CubitUniProjectile.CubitUniProjectile_C" (Transformation|GetWorldTransform (Variables|Default|GetMuzzleScene)) "Undefined" "MultiplyWithRoot" 0 3e+04 true true false "NewEnumerator1" 0 "NewEnumerator0" true self)
  (return))